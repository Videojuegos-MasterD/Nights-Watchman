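; Base interactive object Blueprint that registers itself with the player when the MainCharacter enters its Box trigger.
; On begin overlap it sets itself as the character's InteractiveObject and shows the advice prompt on the PlayerUI widget.
; On end overlap it clears that reference and hides the prompt.
; The UI is found through a top-level GetAllWidgetsOfClass lookup, taking the first result.
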(event `self.Box.OnComponentBeginOverlap`
  (params (OverlappedComponent :type "PrimitiveComponent Object Reference") (OtherActor :type "Actor Object Reference") (OtherComp :type "PrimitiveComponent Object Reference") (OtherBodyIndex :type Integer) (bFromSweep :type Boolean) (SweepResult :type "HitResult Structure (by ref)"))
  ;[1 0.5216 0.5216] Join collision
  (bind _asmain_character (cast `/Game/Blueprints/MainCharacter` OtherActor))
  (set `/Game/Blueprints/MainCharacter.InteractiveObject` self _asmain_character)
  (bind _foundwidgets (`WidgetBlueprintLibrary.GetAllWidgetsOfClass` "/Game/Blueprints/Widgets/PlayerUI.PlayerUI_C"))
  (`/Game/Blueprints/Widgets/PlayerUI.ShowAdvice` (`|GetArrayItem` _foundwidgets) true))

(event `self.Box.OnComponentEndOverlap`
  (params (OverlappedComponent :type "PrimitiveComponent Object Reference") (OtherActor :type "Actor Object Reference") (OtherComp :type "PrimitiveComponent Object Reference") (OtherBodyIndex :type Integer))
  ;[1 0.5216 0.5216] Exit collision
  (bind _asmain_character (cast `/Game/Blueprints/MainCharacter` OtherActor))
  (set `/Game/Blueprints/MainCharacter.InteractiveObject` null _asmain_character)
  (bind _foundwidgets (`WidgetBlueprintLibrary.GetAllWidgetsOfClass` "/Game/Blueprints/Widgets/PlayerUI.PlayerUI_C"))
  (`/Game/Blueprints/Widgets/PlayerUI.ShowAdvice` (`|GetArrayItem` _foundwidgets) false))

(fn `UserConstructionScript`)