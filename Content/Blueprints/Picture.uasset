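; Interactive museum picture that moves the player's camera in for a close look and back out on the next interaction.
; InteractiveEvent toggles on LookPicture, clearing and restoring the character's InteractiveObject to gate input while viewing.
; The first view adds spectrum text, voice audio, dialogue and a delayed skip prompt, while later views only fade in bird ambience.
; Leaving fades out audio and hides dialogue, with a DoOnce triggering the MuseumEffectObject event.
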(event `/Game/Blueprints/InteractiveEvent.InteractiveEvent`
  (bind _spectrumvoice (`self.SpectrumVoice`))
  (bind _asmain_character (cast `/Game/Blueprints/MainCharacter` (`GameplayStatics.GetPlayerCharacter` 0) :!pure true))
  ;[0.0902 0.02353 1] See picture main event
  (bind _foundwidgets (`WidgetBlueprintLibrary.GetAllWidgetsOfClass` "/Game/Blueprints/Widgets/PlayerUI.PlayerUI_C"))
  (`/Game/Blueprints/Widgets/PlayerUI.ShowAdvice` (`|GetArrayItem` _foundwidgets) false)
  (if (`self.LookPicture?`)
    (set `/Game/Blueprints/MainCharacter.InteractiveObject` null _asmain_character)
    (set `/Game/Blueprints/MainCharacter.FinalCameraTransform` (`SceneComponent.K2_GetComponentToWorld` (`self.CameraPosition`)) _asmain_character)
    (`/Game/Blueprints/MainCharacter.CameraToPicture` _asmain_character true)
    (`KismetSystemLibrary.Delay` 1.0)
    (if (`self.FirstTime?`)
      (set `self.FirstTime?` false)
      (bind _returnvalue (`GameplayStatics.SpawnSound2D` "/Game/ThirdParty/StarterContent/Audio/Starter_Birds01.Starter_Birds01" 0.1 1.0 0.0 null))
      (bind _output_get (set `self.AmbienceSound` _returnvalue))
      (`AudioComponent.FadeIn` _output_get 3.0 1.0 0.0 "Linear")
      (bind _foundwidgets_2 (`WidgetBlueprintLibrary.GetAllWidgetsOfClass` "/Game/Blueprints/Widgets/PicturesMainUI.PicturesMainUI_C"))
      (`/Game/Blueprints/Widgets/PicturesMainUI.ShowSpectrumTextBox` (`|GetArrayItem` _foundwidgets_2) true)
      (`KismetSystemLibrary.Delay` 1.0)
      (bind _returnvalue_2 (`GameplayStatics.SpawnSound2D` "/Game/ThirdParty/StarterContent/Audio/Starter_Music01.Starter_Music01" 0.1 1.0 0.0 null))
      (bind _output_get_2 (set `self.SpectrumVoice` _returnvalue_2))
      (`AudioComponent.FadeIn` _output_get_2 3.0 1.0 0.0 "Linear")
      (bind _foundwidgets_3 (`WidgetBlueprintLibrary.GetAllWidgetsOfClass` (`self.DialogueWidgetClass`)))
      (message `/Game/Blueprints/DialogueSequence.ShowDialogue` (`|GetArrayItem` _foundwidgets_3) true)
      (`KismetSystemLibrary.Delay` (`self.DelayToSkip`))
      (set `self.LookPicture?` false)
      (set `/Game/Blueprints/MainCharacter.InteractiveObject` self _asmain_character)
      (bind _foundwidgets_4 (`WidgetBlueprintLibrary.GetAllWidgetsOfClass` "/Game/Blueprints/Widgets/PicturesMainUI.PicturesMainUI_C"))
      (`/Game/Blueprints/Widgets/PicturesMainUI.ShowSkipAdvice` (`|GetArrayItem` _foundwidgets_4) true)
      (else
        (set `self.LookPicture?` false)
        (set `/Game/Blueprints/MainCharacter.InteractiveObject` self _asmain_character)
        (bind _returnvalue_3 (`GameplayStatics.SpawnSound2D` "/Game/ThirdParty/StarterContent/Audio/Starter_Birds01.Starter_Birds01" 0.1 1.0 0.0 null))
        (bind _output_get_3 (set `self.AmbienceSound` _returnvalue_3))
        (`AudioComponent.FadeIn` _output_get_3 3.0 1.0 0.0 "Linear")))
    (else
      (`KismetSystemLibrary.Delay` 0.5)
      (`/Game/Blueprints/MainCharacter.CameraToPicture` (cast `/Game/Blueprints/MainCharacter` (`GameplayStatics.GetPlayerCharacter` 0) :!pure true) false)
      (set `/Game/Blueprints/MainCharacter.InteractiveObject` null _asmain_character)
      (set `self.LookPicture?` true)
      (`/Engine/EditorBlueprintResources/StandardMacros.IsValid` _spectrumvoice
        (:`Is Valid`
          (`AudioComponent.FadeOut` _spectrumvoice 1.0 0.0 "Linear"))
        (:`Is Not Valid`
          _))
      (`AudioComponent.FadeOut` (`self.AmbienceSound`) 3.0 0.0 "Linear")
      (bind _foundwidgets_5 (`WidgetBlueprintLibrary.GetAllWidgetsOfClass` (`self.DialogueWidgetClass`)))
      (message `/Game/Blueprints/DialogueSequence.ShowDialogue` (`|GetArrayItem` _foundwidgets_5) false)
      (`/Engine/EditorBlueprintResources/StandardMacros.DoOnce` false
        (:`Completed`
          (bind _foundwidgets_6 (`WidgetBlueprintLibrary.GetAllWidgetsOfClass` "/Game/Blueprints/Widgets/PicturesMainUI.PicturesMainUI_C"))
          (`/Game/Blueprints/Widgets/PicturesMainUI.ShowSkipAdvice` (`|GetArrayItem` _foundwidgets_6) false)
          (`KismetSystemLibrary.Delay` 1.0)
          (message `/Game/Blueprints/MuseumEffects.EffectEvent` (`self.MuseumEffectObject`)))))))

(fn `UserConstructionScript`
  (`parent.UserConstructionScript`))