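; MusicManager Blueprint that starts and stops the horror ambience main theme and a spectrum voice sound.
; Two events each take a Play flag, spawning a 2D sound, storing it and fading it in, or fading the stored component out.
; The theme's branches each pass through a DoOnce with no visible reset, while the spectrum voice spawns anew on every play call, starting partway into the clip.
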(event `PlayMainTheme`
  (params (`Play?` :type Boolean))
  ;[0.6343 0.2289 1] Play main theme event
  (if `Play?`
    (`/Engine/EditorBlueprintResources/StandardMacros.DoOnce` false
      (:`Completed`
        (bind _returnvalue (`GameplayStatics.SpawnSound2D` "/Game/Audio/Horror_ambience_Theme.Horror_ambience_Theme" 0.1 1.0 0.0 null))
        (bind _output_get (set `self.MainTheme` _returnvalue))
        (`AudioComponent.FadeIn` _output_get 1.0 1.5 0.0 "Linear")))
    (else
      (`/Engine/EditorBlueprintResources/StandardMacros.DoOnce` false
        (:`Completed`
          (`AudioComponent.FadeOut` (`self.MainTheme`) 1.0 0.0 "Linear"))))))

(event `PlaySpectrumSound`
  (params (`Play?` :type Boolean))
  ;[0.6343 0.2289 1] Play spectrum sound event
  (if `Play?`
    (bind _returnvalue (`GameplayStatics.SpawnSound2D` "/Game/Audio/SpectrumVoice.SpectrumVoice" 0.1 1.0 15.0 null))
    (bind _output_get (set `self.SpectrumVoice` _returnvalue))
    (`AudioComponent.FadeIn` _output_get 1.0 1.0 0.0 "Linear")
    (else
      (`AudioComponent.FadeOut` (`self.SpectrumVoice`) 1.0 0.0 "Linear"))))

(fn `UserConstructionScript`)