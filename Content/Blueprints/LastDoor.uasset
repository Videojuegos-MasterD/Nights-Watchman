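; LastDoor is an interactive door that opens once and later shuts once as the player passes its exit triggers.
; Interacting opens it, destroys its Box component and triggers the MainCharacter's FinalRoomAnim.
; Three overlap boxes share one DoOnce, so the first one the MainCharacter enters closes the door.
; OpenCloseDoor drives both motions with timelines that lerp the Pivot's world rotation to fixed angles, with sounds.
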(event `/Game/Blueprints/InteractiveEvent.InteractiveEvent`
  ;[0.0902 0.02353 1] Interactive event
  (`/Engine/EditorBlueprintResources/StandardMacros.DoOnce` false
    (:`Completed`
      (`self.OpenCloseDoor` true)
      (`ActorComponent.K2_DestroyComponent` (`self.Box`))
      (`/Game/Blueprints/MainCharacter.FinalRoomAnim` (cast `/Game/Blueprints/MainCharacter` (`GameplayStatics.GetPlayerCharacter` 0) :!pure true)))))

(event `self.Box1.OnComponentBeginOverlap`
  (params (OverlappedComponent :type "PrimitiveComponent Object Reference") (OtherActor :type "Actor Object Reference") (OtherComp :type "PrimitiveComponent Object Reference") (OtherBodyIndex :type Integer) (bFromSweep :type Boolean) (SweepResult :type "HitResult Structure (by ref)"))
  ;[1 0.5216 0.5216] Exit room collisions
  (cast `/Game/Blueprints/MainCharacter` OtherActor)
  (`/Engine/EditorBlueprintResources/StandardMacros.DoOnce` false :!label _label
    (:`Completed`
      (`self.OpenCloseDoor` false))))

(event `OpenCloseDoor`
  (params (`Open?` :type Boolean))
  (bind _returnvalue (`self.K2_GetActorLocation`))
  ;[1 0.2549 0.08627] Door opening/closing animation
  (set `self.DoorCurrentRotation` (`SceneComponent.K2_GetComponentRotation` (`self.Pivot`)))
  (if `Open?`
    (set `self.DoorTargetRotation` (struct :`Yaw` 180.0))
    (`GameplayStatics.PlaySoundAtLocation` "/Game/Audio/OpenignDoor.OpenignDoor" _returnvalue (struct) 1.0 0.5 0.2 null null null)
    (bind (_direction _alpha) (`Timeline|OpenDoorAnim` :!via `PlayFromStart`)
      (:`Update`
        (`SceneComponent.K2_SetWorldRotation` (`self.Pivot`) (`KismetMathLibrary.RLerp` (`self.DoorCurrentRotation`) (`self.DoorTargetRotation`) _alpha) false false)))
    (else
      (set `self.DoorTargetRotation` (struct :`Yaw` 90.0))
      (`GameplayStatics.PlaySoundAtLocation` "/Game/Audio/OpenignDoor.OpenignDoor" _returnvalue (struct) 1.0 2.5 0.0 null null null)
      (bind (_direction_2 _alpha_2) (`Timeline|CloseDoorAnim` :!via `PlayFromStart`)
        (:`Update`
          (`SceneComponent.K2_SetWorldRotation` (`self.Pivot`) (`KismetMathLibrary.RLerp` (`self.DoorCurrentRotation`) (`self.DoorTargetRotation`) _alpha_2 true) false false))
        (:`Finished`
          (`GameplayStatics.PlaySoundAtLocation` "/Game/Audio/ClosingDoor.ClosingDoor" (`self.K2_GetActorLocation`) (struct) 1.0 1.0 0.1 null null null))))))

(event `self.Box2.OnComponentBeginOverlap`
  (params (OverlappedComponent :type "PrimitiveComponent Object Reference") (OtherActor :type "Actor Object Reference") (OtherComp :type "PrimitiveComponent Object Reference") (OtherBodyIndex :type Integer) (bFromSweep :type Boolean) (SweepResult :type "HitResult Structure (by ref)"))
  ;[1 0.5216 0.5216] Exit room collisions
  (cast `/Game/Blueprints/MainCharacter` OtherActor)
  (goto _label))

(event `self.Box3.OnComponentBeginOverlap`
  (params (OverlappedComponent :type "PrimitiveComponent Object Reference") (OtherActor :type "Actor Object Reference") (OtherComp :type "PrimitiveComponent Object Reference") (OtherBodyIndex :type Integer) (bFromSweep :type Boolean) (SweepResult :type "HitResult Structure (by ref)"))
  ;[1 0.5216 0.5216] Exit room collisions
  (cast `/Game/Blueprints/MainCharacter` OtherActor)
  (goto _label))

(fn `UserConstructionScript`
  (`parent.UserConstructionScript`))