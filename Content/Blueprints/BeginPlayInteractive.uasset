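; BeginPlayInteractive is an interactive object that serves as the player's first interaction when play begins, used to skip the first dialogue.
; On BeginPlay it registers itself as the MainCharacter's InteractiveObject.
; Its InteractiveEvent calls InteractiveEventMessage on the first top-level PlayerUI widget and clears that reference.
; After a short delay it sets CanMove to true on the character.
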(event `self.ReceiveBeginPlay`
  ;[0 0.4217 1] Set this object to the first interactive object
  (set `/Game/Blueprints/MainCharacter.InteractiveObject` self (cast `/Game/Blueprints/MainCharacter` (`GameplayStatics.GetPlayerCharacter` 0) :!pure true)))

(event `/Game/Blueprints/InteractiveEvent.InteractiveEvent`
  (bind _asmain_character (cast `/Game/Blueprints/MainCharacter` (`GameplayStatics.GetPlayerCharacter` 0) :!pure true))
  ;[1 0.6902 0.01961] Skips the first dialogue
  (bind _foundwidgets (`WidgetBlueprintLibrary.GetAllWidgetsOfClass` "/Game/Blueprints/Widgets/PlayerUI.PlayerUI_C"))
  (message `/Game/Blueprints/InteractiveEvent.InteractiveEvent` (`|GetArrayItem` _foundwidgets))
  (set `/Game/Blueprints/MainCharacter.InteractiveObject` null _asmain_character)
  (`KismetSystemLibrary.Delay` 1.0)
  (set `/Game/Blueprints/MainCharacter.CanMove?` true _asmain_character))

(fn `UserConstructionScript`
  (`parent.UserConstructionScript`))